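; BP_lever is a grabbable lever that rotates to follow the motion controller holding it.
; Its GrabComponent stores the controller on grab and clears it on drop.
; While held, Tick converts the look-at pitch from mesh to controller, with a fixed offset, into a roll clamped between Min and Max.
; It broadcasts that angle remapped to 0–1 through OnRotating and prints a debug string each frame.
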(event OnGrabbed(GrabComponent)
  (params (MotionController :type Motion%20Controller%20Component%20Object%20Reference))
  (Variables|Default|SetMotion%20Controller MotionController))

(event OnDropped(GrabComponent)
  (params (MotionController :type Motion%20Controller%20Component%20Object%20Reference))
  (if (== MotionController (Variables|Default|GetMotion%20Controller))
    (Variables|Default|SetMotion%20Controller 0)))

(event EventTick
  (params (DeltaSeconds :type Float%20%28single-precision%29))
  (bind _motion_controller (Variables|Default|GetMotion%20Controller)
    (:then
      (Development|PrintString "rotating")
      (Transformation|SetRelativeRotation (Variables|Default|GetStaticMesh) (Math|Rotator|MakeRotator (Math|Float|Clamp(Float) (+ (.pitch (Math|Rotator|FindLookatRotation (.location (Transformation|GetWorldTransform (Variables|Default|GetStaticMesh))) (.location (Transformation|GetWorldTransform _motion_controller)))) -5e+01) (Variables|Default|GetMin) (Variables|Default|GetMax)) 0.0 0.0) false false)
      (Default|CallOnRotating (Math|Float|MapRangeClamped (Math|Float|Clamp(Float) (+ (.pitch (Math|Rotator|FindLookatRotation (.location (Transformation|GetWorldTransform (Variables|Default|GetStaticMesh))) (.location (Transformation|GetWorldTransform _motion_controller)))) -5e+01) (Variables|Default|GetMin) (Variables|Default|GetMax)) (Variables|Default|GetMin) (Variables|Default|GetMax) 0.0 1.0)))
    (:else)))

(fn ConstructionScript)

(fn OnRotating
  (params (Angle :type Float%20%28single-precision%29)))