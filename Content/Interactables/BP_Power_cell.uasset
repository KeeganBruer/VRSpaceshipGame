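; Power cell interactable that shows a charged or uncharged look based on its status.
; On BeginPlay it applies its initial status through SetStatus, which overrides and first calls the parent version.
; SetStatus then swaps the mesh's second material slot to the charged material for status 1, also printing a debug "Hello", or to the uncharged material otherwise.
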(event EventBeginPlay
  (|CallParentFunction)
  (CallFunction|SetStatus (Variables|Default|GetinitStatus)))

(event Collision|EventActorBeginOverlap
  (params (OtherActor :type Actor%20Object%20Reference))
  (|CallParentFunction OtherActor) ; This node is disabled and will not be called.\nDrag off pins to build functionality.
)

(event EventTick
  (params (DeltaSeconds :type Float%20%28single-precision%29))
  (|CallParentFunction DeltaSeconds) ; This node is disabled and will not be called.\nDrag off pins to build functionality.
)

(fn ConstructionScript
  (|CallParentFunction))

(fn SetStatus
  (params (NewStatus :type String))
  (|CallParentFunction NewStatus)
  (if (Utilities|Enum|Equal(Enum) NewStatus "1")
    (Development|PrintString "Hello")
    (Rendering|Material|SetMaterial (Variables|Character|GetMesh) 1 (Variables|Default|GetChargedMat))
    (else
      (Rendering|Material|SetMaterial (Variables|Character|GetMesh) 1 (Variables|Default|GetUnchargedMat)))))